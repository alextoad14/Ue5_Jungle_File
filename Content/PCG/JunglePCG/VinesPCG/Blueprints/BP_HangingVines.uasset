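; Hanging vines actor for the jungle PCG set that hosts static meshes and a PCG component.
; The construction script adds a component per StaticMesh array entry, assigning the mesh and tags, including MossOn, only when the entry is valid.
; The Redo event forces the PCG component to regenerate; the file does not otherwise connect it to the tagged meshes.
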(event Custom|Redo
  (PCG|Generate (Variables|Default|GetPCG) true))

(event EventBeginPlay)

(event Collision|EventActorBeginOverlap
  (params (OtherActor :type Actor%20Object%20Reference)))

(event EventTick
  (params (DeltaSeconds :type Float%20%28single-precision%29)))

(fn ConstructionScript
  (for _array_element (Variables|Default|GetStaticMesh)
    (bind _returnvalue (AddComponent|AddStaticMeshComponent false))
    (Utilities|IsValid _array_element
      (:Is%20Valid
        (Components|StaticMesh|SetStaticMesh _returnvalue _array_element)
        (Variables|/Script/Engine.ActorComponent|SetComponentTags _returnvalue (Utilities|Array|MakeArray "MossOn" "ThisWorked"))))))